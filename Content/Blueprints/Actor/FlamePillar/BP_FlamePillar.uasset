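; BP_FlamePillar is a flame pillar actor that makes its fire light flicker.
; From BeginPlay it randomly plays one of two FlameIntensity timelines and picks again whenever one finishes, so the flicker loops without a fixed pattern.
; Each timeline update passes its curve value to ScaleFlameIntensity, which multiplies it by BaseIntensity and applies it to FireLight.
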(event `self.ReceiveBeginPlay`
  (`self.Chosetimeline`))

(event `Chosetimeline`
  (switch `int` (`KismetMathLibrary.RandomIntegerInRange` 0 1)
    (:`Default`
      (`self.Timeline2` :!label _label))
    (:`0`
      (`self.Timeline1`))
    (:`1`
      (goto _label))))

(event `Timeline1`
  (bind (_direction _flameintensity) (`Timeline|FlameIntensity1` :!via `PlayFromStart`)
    (:`Update`
      (`self.Scale Flame Intensity` _flameintensity))
    (:`Finished`
      (`self.Chosetimeline`))))

(event `Timeline2`
  (bind (_direction _flameintensity) (`Timeline|FlameIntensity2` :!via `PlayFromStart`)
    (:`Update`
      (`self.Scale Flame Intensity` _flameintensity))
    (:`Finished`
      (`self.Chosetimeline`))))

(fn `Scale Flame Intensity`
  (params (Intensity :type "Float (double-precision)"))
  (`LightComponent.SetIntensity` (`self.FireLight`) (* Intensity (`self.BaseIntensity`))))

(fn `UserConstructionScript`)