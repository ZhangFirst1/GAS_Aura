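; Fireball actor for the FireBlast ability that flies out, returns to an actor and explodes near it.
; On authority, two timelines lerp its location to a forward apex, then back to ReturnToActor's current position.
; Within explode distance, it calls OnHit, applies radial damage to nearby live players with death impulse and knockback pitched to 45 degrees, then destroys itself.
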(event `self.StartOutgoingTimeline`
  (bind _array (`|MakeArray` (`self.GetOwner`)))
  (`/Engine/EditorBlueprintResources/ActorMacros.Switch Has Authority`
    (:`Authority`
      ;[1 1 1] 存储初始和最远位置
      (set `self.InitialLocation` (`self.K2_GetActorLocation`))
      (set `self.ApexLocation` (+ (`self.InitialLocation`) (* (`self.GetActorForwardVector`) (`self.TravelDistance`))))
      (bind (_direction _outgoingtrack) (`Timeline|OutgoingTimeline`)
        (:`Update`
          ;[1 1 1] 使用OutgoingTimeline在初始和最远位置做混合，并更新火球位置
          (`self.K2_SetActorLocation` (`KismetMathLibrary.VLerp` (`self.InitialLocation`) (`self.ApexLocation`) _outgoingtrack)))
        (:`Finished`
          ;[1 1 1] 使用ReturningTimeline在最远和返回Actor位置做混合，并更新火球位置
          (bind (_direction_2 _returningtrack) (`Timeline|ReturningTimeline`)
            (:`Update`
              (`self.K2_SetActorLocation` (`KismetMathLibrary.VLerp` (`self.ApexLocation`) (`self.K2_GetActorLocation` (`self.ReturnToActor`)) _returningtrack))
              ;[1 1 1] 当前火球位置是否在爆炸范围内
              (if (`self.IsWithinExplodeDistance`)
                ;[1 1 1] 爆炸逻辑，会调用GC，同时设置爆炸伤害参数
                (`self.OnHit`)
                (`AuraAbilitySystemLibrary.SetIsRadialDamageEffectParam` (`self.ExplosionDamageParams`) true (`self.RadialDamageInnerRadius`) (`self.RadialDamageOuterRadius`) (`self.K2_GetActorLocation`))
                ;[1 1 1] 获取周围的Actor（忽略自身）
                (`KismetArrayLibrary.Array_Add` _array self)
                (bind _outoverlappingactors (`AuraAbilitySystemLibrary.GetLivePlayersWithinRadius` self _array (`self.RadialDamageOuterRadius`) (`self.K2_GetActorLocation`)))
                (for _array_element _outoverlappingactors
                  ;[1 1 1] 对爆炸范围内的每个Actor造成伤害和击退
                  (`AuraAbilitySystemLibrary.SetTargetEffectParamsASC` (`self.ExplosionDamageParams`) (`AbilitySystemBlueprintLibrary.GetAbilitySystemComponent` _array_element))
                  (set `self.KnockbackDirection` (- (`self.K2_GetActorLocation` _array_element) (`self.K2_GetActorLocation`)))
                  (`AuraAbilitySystemLibrary.SetKnockbackDirection` (`self.ExplosionDamageParams`) (`self.OverrideKnockbackPitch`) (`self.KnockbackMagnitude`))
                  (`AuraAbilitySystemLibrary.SetDeathImpulseDirection` (`self.ExplosionDamageParams`) (`self.KnockbackDirection`) (`self.DeathImpulseMagnitude`))
                  (`AuraAbilitySystemLibrary.ApplyDamageEffect` (`self.ExplosionDamageParams`)))
                (`self.K2_DestroyActor`)))))))))

(fn `IsWithinExplodeDistance`
  (returns (ReturnValue :type Boolean))
  (return (<= (`KismetMathLibrary.VSize` (- (`self.K2_GetActorLocation`) (`self.K2_GetActorLocation` (`self.ReturnToActor`)))) (`self.ExplodeDistance`))))

(fn `OverrideKnockbackPitch`
  (returns (ReturnValue :type "Vector Structure"))
  (bind (_returnvalue_roll _returnvalue_pitch _returnvalue_yaw) (`KismetMathLibrary.BreakRotator` (`KismetMathLibrary.MakeRotFromX` (`self.KnockbackDirection`))))
  (return (`KismetMathLibrary.GetForwardVector` (`KismetMathLibrary.MakeRotator` _returnvalue_roll 45.0 _returnvalue_yaw))))

(fn `UserConstructionScript`)